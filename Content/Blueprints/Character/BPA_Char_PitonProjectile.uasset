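; Piton projectile actor that sticks where it hits and can be retracted to the player.
; On a hit while not retracting, it stops projectile movement and disables mesh physics and collision.
; Retract re-enables both and launches the mesh toward the player with a single velocity-change impulse.
; While retracting, Tick destroys it once its distance to the player stops shrinking and plays a lock sound at the player.
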(event OnComponentHit(StaticMesh)
  (params (HitComponent :type Primitive%20Component%20Object%20Reference) (OtherActor :type Actor%20Object%20Reference) (OtherComp :type Primitive%20Component%20Object%20Reference) (NormalImpulse :type Vector :default "0, 0, 0") (Hit :type Hit%20Result%20Structure%20%28by%20ref%29))
  (bind _staticmesh (Variables|Default|GetStaticMesh))
  (if (not (Variables|Default|GetIsRetracting))
    (Components|Movement|StopMovementImmediately (Variables|Default|GetProjectileMovement))
    (Physics|SetSimulatePhysics _staticmesh false)
    (Collision|SetCollisionEnabled _staticmesh "NoCollision")))

(event EventBeginPlay)

(event Collision|EventActorBeginOverlap
  (params (OtherActor :type Actor%20Object%20Reference)))

(event EventTick
  (params (DeltaSeconds :type Float%20%28single-precision%29))
  (bind _returnvalue (Transformation|GetActorLocation))
  (bind _returnvalue_2 (Game|GetPlayerCharacter 0))
  (bind _returnvalue_3 (Transformation|GetActorLocation _returnvalue_2))
  (bind _returnvalue_4 (Math|Vector|Distance(Vector) _returnvalue_3 _returnvalue))
  (if (Variables|Default|GetIsRetracting)
    ;[1 1 1] Update distance between piton and player if smaller, else destroy piton since it's moving away form player
    (if (< _returnvalue_4 (Variables|Default|GetLastDistanceBetweenPitonAndPlayer))
      (Variables|Default|SetLastDistanceBetweenPitonAndPlayer _returnvalue_4)
      (else
        (Actor|DestroyActor)
        (Audio|PlaySoundatLocation "/Game/Audio/PitonLock.PitonLock" (Transformation|GetActorLocation (Game|GetPlayerCharacter 0)) "0, 0, 0" 1.0 1.0 0.0 0 0 0)))))

(fn ConstructionScript)

(fn Retract
  (bind _staticmesh (Variables|Default|GetStaticMesh))
  (Variables|Default|SetIsRetracting true)
  (Physics|SetSimulatePhysics _staticmesh true)
  (Collision|SetCollisionEnabled _staticmesh "QueryAndPhysics")
  (bind _returnvalue (CallFunction|GetDirectionfromPitontoPlayer))
  (Physics|AddImpulse (Variables|Default|GetStaticMesh) (* _returnvalue (Variables|Default|GetRetractSpeed)) "None" true)
  (Variables|Default|SetRetractionImpulseHasBeenAdded true))

(fn GetDirectionfromPitontoPlayer
  (return (Math|Vector|Normalize (- (Transformation|GetActorLocation (Game|GetPlayerCharacter 0)) (Transformation|GetActorLocation)))))